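; Weather system actor that runs a looping 24-hour day/night cycle, rotating the sun by curve over a configurable day length.
; Each tick, UpdateWeather blends sun, skylight and sky atmosphere between sunny and cloudy using a time-based weather curve.
; Curves also drive fog and toggle optional rain and snow; light shafts run only in daytime.
; The construction script previews this in-editor; only snow attaches to the player, as rain's attach is unwired.
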(event EventBeginPlay
  (Variables|Default|SetOneHour (/ (* (Variables|Default|GetDayLengthInMinutes) 6e+01) 24.0))
  (Transformation|AttachComponentToComponent (Variables|Default|GetSnowComponent) (Variables|/Script/Engine.Actor|GetRootComponent (Game|Player|GetPlayerPawn 0)) "None" "SnapToTarget" "KeepRelative" "KeepRelative" true))

(event EventTick
  (params (DeltaSeconds :type Float%20%28single-precision%29))
  (if (> (+ (Math|Float|SafeDivide DeltaSeconds (Variables|Default|GetOneHour)) (Variables|Default|GetCurrentTime) 0.0) 0.0)
    (if (<= (+ (Math|Float|SafeDivide DeltaSeconds (Variables|Default|GetOneHour)) (Variables|Default|GetCurrentTime) 0.0) 24.0)
      (Variables|Default|SetCurrentTime (+ (Math|Float|SafeDivide DeltaSeconds (Variables|Default|GetOneHour)) (Variables|Default|GetCurrentTime) 0.0))
      (else
        (Variables|Default|SetCurrentTime (Math|Float|Absolute(Float) (- 24.0 (+ (Math|Float|SafeDivide DeltaSeconds (Variables|Default|GetOneHour)) (Variables|Default|GetCurrentTime) 0.0))))))
    (Transformation|SetActorRotation (Variables|Default|GetSun) (Math|Rotator|MakeRotator 0.0 (Math|Curves|GetFloatValue (Variables|Default|GetDayLengthCurve) (Variables|Default|GetCurrentTime)) 0.0))
    (CallFunction|UpdateWeather)))

(fn ConstructionScript
  (Transformation|SetActorLocation (Math|Conversions|ToVector(Float) (Class|GameplayStatics|GetWorldOriginLocation)) false false)
  (Utilities|IsValid (Variables|Default|GetSun)
    (:Is%20Valid
      (Utilities|IsValid (Variables|Default|GetSkyLight)
        (:Is%20Valid
          (Utilities|IsValid (Variables|Default|GetSkyAtmosphere)
            (:Is%20Valid
              (Utilities|IsValid (Variables|Default|GetFog)
                (:Is%20Valid
                  (Transformation|SetActorRotation (Variables|Default|GetSun) (Math|Rotator|MakeRotator 0.0 (Math|Curves|GetFloatValue (Variables|Default|GetDayLengthCurve) (Variables|Default|GetCurrentTime)) 0.0))
                  (CallFunction|UpdateWeather))))))))))

(fn UpdateWeather
  (bind _sunintensitycurve (Variables|Default|GetSunIntensityCurve))
  (bind _skylightintensitycurve (Variables|Default|GetSkylightIntensityCurve))
  (bind _currenttime (Variables|Default|GetCurrentTime))
  (bind _sun (Variables|Default|GetSun))
  (bind _currenttime_2 (Variables|Default|GetCurrentTime))
  (bind _rayleighdistributioncurve (Variables|Default|GetRayleighDistributionCurve))
  (bind _currenttime_3 (Variables|Default|GetCurrentTime))
  (bind _currenttime_4 (Variables|Default|GetCurrentTime))
  (bind _returnvalue (Math|Curves|GetVectorValue _skylightintensitycurve _currenttime))
  (bind _returnvalue_2 (Actor|GetComponentbyClass _sun "/Script/Engine.DirectionalLightComponent"))
  (bind _returnvalue_3 (Math|Curves|GetVectorValue _rayleighdistributioncurve _currenttime_3))
  (bind _returnvalue_4 (Math|Curves|GetVectorValue _sunintensitycurve _currenttime_4))
  (LocalVariables|SetWeatherType (Math|Curves|GetFloatValue (Variables|Default|GetWeatherTypeCurve) (Variables|Default|GetCurrentTime)))
  (Rendering|Components|Light|SetIntensity (Variables|/Script/Engine.Light|GetLightComponent (Variables|Default|GetSun)) (Math|Float|Lerp (.x _returnvalue_4) (.y _returnvalue_4) (LocalVariables|GetWeatherType)))
  (Rendering|Components|Light|SetIntensity (Variables|/Script/Engine.SkyLight|GetLightComponent (Variables|Default|GetSkyLight)) (Math|Float|Lerp (.x _returnvalue) (.y _returnvalue) (LocalVariables|GetWeatherType)))
  (if (Variables|Default|GetbRain)
    (if (Math|Float|NearlyEqual(Float) (Math|Curves|GetFloatValue (Variables|Default|GetRainTimelineCurve) (Variables|Default|GetCurrentTime)) 1.0 1e-06)
      (Components|Activation|Activate (Variables|Default|GetRainComponent) false)
      (else
        (Components|Activation|Deactivate (Variables|Default|GetRainComponent))))
    (else
      (Components|Activation|Deactivate (Variables|Default|GetRainComponent))))
  (if (Variables|Default|GetbSnow)
    (if (Math|Float|NearlyEqual(Float) (Math|Curves|GetFloatValue (Variables|Default|GetSnowTimelineCurve) (Variables|Default|GetCurrentTime)) 1.0 1e-06)
      (Components|Activation|Activate (Variables|Default|GetSnowComponent) false)
      (else
        (Components|Activation|Deactivate (Variables|Default|GetSnowComponent))))
    (else
      (Components|Activation|Deactivate (Variables|Default|GetSnowComponent))))
  (if (Variables|Default|GetbFog)
    (Class|ExponentialHeightFogComponent|SetFogDensity (Variables|/Script/Engine.ExponentialHeightFog|GetComponent (Variables|Default|GetFog)) (Math|Curves|GetFloatValue (Variables|Default|GetFogTimelineCurve) (Variables|Default|GetCurrentTime)))
    (Class|ExponentialHeightFogComponent|SetFogHeightFalloff (Variables|/Script/Engine.ExponentialHeightFog|GetComponent (Variables|Default|GetFog)) (Math|Curves|GetFloatValue (Variables|Default|GetFogHeightFalloffCurve) (Variables|Default|GetCurrentTime)))
    (else
      (Class|ExponentialHeightFogComponent|SetFogDensity (Variables|/Script/Engine.ExponentialHeightFog|GetComponent (Variables|Default|GetFog)) 0.001)
      (Class|ExponentialHeightFogComponent|SetFogHeightFalloff (Variables|/Script/Engine.ExponentialHeightFog|GetComponent (Variables|Default|GetFog)) 0.2)))
  (if (and (> _currenttime_2 6.0) (< _currenttime_2 18.0))
    (Class|DirectionalLightComponent|SetEnableLightShaftOcclusion _returnvalue_2 true)
    (Class|LightComponent|SetEnableLightShaftBloom _returnvalue_2 true)
    (else
      (Class|DirectionalLightComponent|SetEnableLightShaftOcclusion _returnvalue_2 false)
      (Class|LightComponent|SetEnableLightShaftBloom _returnvalue_2 false)))
  (Class|SkyAtmosphereComponent|SetRayleighExponentialDistribution (Variables|/Script/Engine.SkyAtmosphere|GetSkyAtmosphereComponent (Variables|Default|GetSkyAtmosphere)) (Math|Float|Lerp (.x _returnvalue_3) (.y _returnvalue_3) (LocalVariables|GetWeatherType)))
  (Class|SkyAtmosphereComponent|SetRayleighScattering (Variables|/Script/Engine.SkyAtmosphere|GetSkyAtmosphereComponent (Variables|Default|GetSkyAtmosphere)) (Math|Color|Lerp(LinearColor) (Variables|Default|GetSunnySkyColor) (Variables|Default|GetCloudySkyColor) (LocalVariables|GetWeatherType))))